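; BP_MonsterSpawner is an actor that spawns monsters at its attached actors once the game starts.
; On BeginPlay it gathers those actors as spawn points and binds to BP_GameMode's game-start event, which begins spawning after a configurable delay.
; A re-armed timer spawns MonsterClass at a random point every three seconds, retrying failed spawns without counting them, until the target count is reached.
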(event Custom|StartSpawning
  ;[0.15 0.15 0.15 0.5] 몬스터 생성
  (Utilities|Time|SetTimerbyEvent (delegate Custom|SpawnMonster) 3.0))

(event Custom|SpawnMonster
  ;[0.15 0.15 0.15 0.5] 몬스터 생성
  (bind _returnvalue (Game|SpawnActorfromClass (Variables|Default|GetMonsterClass) (Transformation|GetActorTransform (.OutItem (Utilities|Array|Random (Variables|Default|GetSpawnPoint)))) "Undefined" "MultiplyWithRoot" 0 0))
  (Utilities|IsValid _returnvalue
    (:Is%20Valid
      ;;[0.15 0.15 0.15 0.5] 최대 생성량 체크
      (bind _result (Math|Integer|IncrementInt (Variables|Default|GetSpawnCnt))
        (:%20%20
          (if (< _result (Variables|Default|GetTargetSpawnCnt))
            (CallFunction|StartSpawning)))))
    (:Is%20Not%20Valid
      (CallFunction|StartSpawning))))

(event Custom|OnGameStart
  (Utilities|FlowControl|Delay (Variables|Default|GetGameStartWaitTime))
  (CallFunction|StartSpawning))

(event EventBeginPlay
  (bind _output_get (Variables|Default|SetSpawnPoint (Actor|GetAttachedActors true false)))
  (if (> (Utilities|Array|Length _output_get) 0)
    (bind _asbp_game_mode (Utilities|Casting|CastToBP_GameMode (Game|GetGameMode)))
    (EventDispatchers|BindEventtoOnGameStart _asbp_game_mode (delegate Custom|OnGameStart))))

(fn ConstructionScript)