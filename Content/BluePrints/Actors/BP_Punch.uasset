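; BP_Punch is an overlap-triggered actor that reacts visually when something touches it.
; Begin overlap sets the StaticMesh material parameter Alpha to 1, then spawns P_Explosion at the actor's location if the other actor is a Character; end overlap resets Alpha to 0.
; An upward PunchPower impulse on the character and the actor's self-destruction are present but disconnected, so neither runs.
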(event EventBeginPlay)

(event Collision|EventActorBeginOverlap
  (params (OtherActor :type Actor%20Object%20Reference))
  (Rendering|Material|SetScalarParameterValueonMaterials (Variables|Default|GetStaticMesh) "Alpha" 1.0)
  ;[0.15 0.15 0.15 0.5] 캐릭터 상승
  (bind _ascharacter (Utilities|Casting|CastToCharacter OtherActor))
  (Effects|SpawnEmitteratLocation "/Game/Particles/P_Explosion.P_Explosion" (Transformation|GetActorLocation)))

(event EventTick
  (params (DeltaSeconds :type Float%20%28single-precision%29)))

(event Collision|EventActorEndOverlap
  (params (OtherActor :type Actor%20Object%20Reference))
  (Rendering|Material|SetScalarParameterValueonMaterials (Variables|Default|GetStaticMesh) "Alpha" 0.0))

(fn ConstructionScript)