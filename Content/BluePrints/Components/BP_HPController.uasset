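; BP_HPController is a health component that tracks HP and signals death through the OnDead event.
; Its ReceiveDmg event subtracts Dmg from HP only when Dmg is zero or negative and HP is non-negative, so positive damage is ignored.
; After that subtraction, it fires OnDead if HP is at or below zero.
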(event Custom|ReceiveDmg
  (params (Dmg :type Float%20%28double-precision%29))
  (if (<= Dmg 0.0)
    (if (>= (Variables|Default|GetHP) 0.0)
      (bind _output_get (Variables|Default|SetHP (- (Variables|Default|GetHP) Dmg)))
      (if (<= _output_get 0.0)
        (Default|CallOnDeadEvent)))))