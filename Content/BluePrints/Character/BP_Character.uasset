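; Player character Blueprint with Enhanced Input movement, camera look and melee combo attacks that require a collected weapon.
; Attack input starts AM_Atk from Locomotion; during Battle it sets NextCombo from the current montage section, and AtkEnd restores Locomotion.
; Collected weapons attach to the WeaponPosition mesh socket and become owned by the character.
; Attack-check begin/end dispatchers, bound on pickup, relay hit-detection windows to the weapon.
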(event Custom|AtkEnd
  ;[0.15 0.15 0.15 0.5] 공격이 종료시 사용 이벤트
  (Variables|Default|SetState_BP "NewEnumerator0"))

(event Custom|OnWeaponCollected
  (params (WeaponActor :type BP%20Weapon%20Object%20Reference))
  ;[0.15 0.15 0.15 0.5] 무기 습득 처리
  (Actor|SetOwner WeaponActor self)
  (Transformation|AttachComponentToComponent WeaponActor (Variables|Character|GetMesh) "WeaponPosition" "SnapToTarget" "SnapToTarget" "SnapToTarget" true)
  (Variables|Default|SetWeaponActor WeaponActor)
  (Variables|Default|SetHasWeapon true)
  ;[1 0 0 0.5] 공격 판정 시작 이벤트에 함수 등록 (구독)
  (EventDispatchers|BindEventtoAtkCheckBeginEvent (delegate Custom|RaiseAtkCheckBegin))
  ;[1 0 0 0.5] 공격 판정 종료 이벤트에 함수 등록 (구독)
  (EventDispatchers|BindEventtoAtkCheckEndEvent (delegate Custom|RaiseAtkCheckEnd)))

(event Custom|OnAtkCheckEnd
  ;[0.15 0.15 0.15 0.5] 공격 판정 종료
  (Default|CallAtkCheckEndEvent))

(event Custom|OnAtkCheckBegin
  ;[0.15 0.15 0.15 0.5] 공격 판정 시작
  (Default|CallAtkCheckBeginEvent))

(event Custom|RaiseAtkCheckBegin
  (bind _weaponactor (Variables|Default|GetWeaponActor))
  ;[1 0 0 0.5] 공격 판정 시작 이벤트에 함수 등록 (구독)
  (Utilities|IsValid _weaponactor
    (:Is%20Valid
      (Default|OnAtkCheckBegin _weaponactor))))

(event Custom|RaiseAtkCheckEnd
  (bind _weaponactor (Variables|Default|GetWeaponActor))
  ;[1 0 0 0.5] 공격 판정 종료 이벤트에 함수 등록 (구독)
  (Utilities|IsValid _weaponactor
    (:Is%20Valid
      (Default|OnAtkCheckEnd _weaponactor))))

(event Input|EnhancedActionEvents|EnhancedInputActionIA_Move
  (params (ActionValue :type Vector%202D%20Structure) (ElapsedSeconds :type Float%20%28double-precision%29) (TriggeredSeconds :type Float%20%28double-precision%29) (InputAction :type Input%20Action%20Object%20Reference :default "/Game/BluePrints/Input/IA_Move.IA_Move"))
  ;[0 0 1 0.5] 캐릭터 이동
  (Pawn|Input|AddMovementInput (Math|Vector|GetRightVector (Pawn|GetControlRotation :!class /Script/Engine.Pawn)) (.x ActionValue) false)
  (Pawn|Input|AddMovementInput (Math|Vector|GetForwardVector (Math|Rotator|MakeRotator 0.0 0.0 (.yaw (Pawn|GetControlRotation :!class /Script/Engine.Pawn)))) (.y ActionValue) false))

(event Input|EnhancedActionEvents|EnhancedInputActionIA_View
  (params (ActionValue :type Vector%202D%20Structure) (ElapsedSeconds :type Float%20%28double-precision%29) (TriggeredSeconds :type Float%20%28double-precision%29) (InputAction :type Input%20Action%20Object%20Reference :default "/Game/BluePrints/Input/IA_View.IA_View"))
  ;[0 0 1 0.5] 카메라 회전
  (Pawn|Input|AddControllerYawInput (.x ActionValue)) ; 마우스 x축 회전, 언리얼 z축 회전을 의미함
  (Pawn|Input|AddControllerPitchInput (.y ActionValue)) ; 마우스 y축 회전, 언리얼 y축 회전을 의미함
)

(event Input|EnhancedActionEvents|EnhancedInputActionIA_Atk
  (params (ActionValue :type Boolean) (ElapsedSeconds :type Float%20%28double-precision%29) (TriggeredSeconds :type Float%20%28double-precision%29) (InputAction :type Input%20Action%20Object%20Reference :default "/Game/BluePrints/Input/IA_Atk.IA_Atk"))
  ;[0.15 0.15 0.15 0.5] 콤보 공격
  (:Started
    (if (Variables|Default|GetHasWeapon)
      ;;[0.15 0.15 0.15 0.5] 일반 상태인지 체크
      (switch Utilities|FlowControl|Switch|SwitchonPlayerState (Variables|Default|GetState_BP)
        (:NewEnumerator0
          (Variables|Default|SetState_BP "NewEnumerator1")
          (Animation|PlayAnimMontage "/Game/BluePrints/Character/AM_Atk.AM_Atk" 1.0 "None"))
        (:NewEnumerator1
          (switch name (Animation|Montage|MontageGetCurrentSection (Components|SkeletalMesh|GetAnimInstance (Variables|Character|GetMesh)) "/Game/BluePrints/Character/AM_Atk.AM_Atk")
            (:Atk1
              (Variables|Default|SetNextCombo "Atk2"))
            (:Atk2
              (Variables|Default|SetNextCombo "Atk3"))
            (:Atk3
              (Variables|Default|SetNextCombo "Atk4"))))))))

(event EventBeginPlay)

(event Collision|EventActorBeginOverlap
  (params (OtherActor :type Actor%20Object%20Reference)))

(event EventTick
  (params (DeltaSeconds :type Float%20%28single-precision%29)))

(fn ConstructionScript)