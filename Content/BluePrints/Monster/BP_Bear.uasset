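; BP_Bear is a bear monster that takes damage and dies with a dissolve effect.
; Damage goes to BPHPController, whose dead event sets the state, disables capsule collision and plays a timeline driving Dissolve and HitValue material parameters before destroying the actor.
; Overlaps with actors tagged PlayerWeapon play a separate hit timeline that drives HitValue on the mesh materials.
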(event Custom|ReceiveOnDead
  (bind _mesh (Variables|Character|GetMesh))
  ;[0.15 0.15 0.15 0.5] Dead 이벤트 바인딩
  (Variables|Default|SetState_BP "NewEnumerator3")
  (Collision|SetCollisionEnabled (Variables|Collision|GetCapsuleComponent) "NoCollision")
  (bind (_direction _dissolve _hitvalue) (Timeline|DeadEffect PlayFromStart)
    (:Update
      (Rendering|Material|SetScalarParameterValueonMaterials _mesh "Dissolve" _dissolve)
      (Rendering|Material|SetScalarParameterValueonMaterials _mesh "HitValue" _hitvalue))
    (:Finished
      (Actor|DestroyActor))))

(event EventBeginPlay
  ;[0.15 0.15 0.15 0.5] Dead 이벤트 바인딩
  (EventDispatchers|BindEventtoOnDeadEvent (Variables|Default|GetBP_HPController) (delegate Custom|ReceiveOnDead)))

(event Collision|EventActorBeginOverlap
  (params (OtherActor :type Actor%20Object%20Reference))
  ;[0.15 0.15 0.15 0.5] 피격 이펙트 처리
  (if (Actor|ActorHasTag OtherActor "PlayerWeapon")
    (bind _hitvalue (Timeline|HitEffect PlayFromStart)
      (:Update
        (Rendering|Material|SetScalarParameterValueonMaterials (Variables|Character|GetMesh) "HitValue" _hitvalue)))))

(event EventTick
  (params (DeltaSeconds :type Float%20%28single-precision%29)))

(event Game|Damage|EventAnyDamage
  (params (Damage :type Float%20%28single-precision%29) (DamageType :type Damage%20Type%20Object%20Reference) (InstigatedBy :type Controller%20Object%20Reference) (DamageCauser :type Actor%20Object%20Reference))
  ;[0.15 0.15 0.15 0.5] 피격에 따른 hp 변화
  (Default|ReceiveDmg (Variables|Default|GetBP_HPController) Damage))

(fn ConstructionScript)